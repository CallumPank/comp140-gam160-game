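; Pickup that temporarily enlarges a player's paddle when a BP_Ball overlaps its sphere.
; On BeginPlay it caches the first P1_Paddle and P2_Paddle in the level.
; The ball's CurrentPlayer picks the paddle, which is stretched along X, then reset after a fixed delay.
; The pickup destroys itself only after that delay; its ChangeScale function, which scales the pickup itself, is not called here.
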(event OnComponentBeginOverlap(Sphere)
  (params (OverlappedComponent :type Primitive%20Component%20Object%20Reference) (OtherActor :type Actor%20Object%20Reference) (OtherComp :type Primitive%20Component%20Object%20Reference) (OtherBodyIndex :type Integer) (bFromSweep :type Boolean) (SweepResult :type Hit%20Result%20Structure%20%28by%20ref%29))
  (bind _asbp_ball (Utilities|Casting|CastToBP_Ball OtherActor))
  (if (== (Variables|/Game/Blueprints/BP_Ball.BP_Ball_C|GetCurrent%20Player _asbp_ball) 1)
    (Transformation|SetActorScale3D (Variables|Default|GetPaddle%201) "2.000000,1.000000,1.000000")
    (Utilities|FlowControl|Delay 7.0)
    (Transformation|SetActorScale3D (Variables|Default|GetPaddle%201) "1.000000,1.000000,1.000000")
    (else
      (Transformation|SetActorScale3D (Variables|Default|GetPaddle%202) "2.000000,1.000000,1.000000")
      (Utilities|FlowControl|Delay 7.0)
      (Transformation|SetActorScale3D (Variables|Default|GetPaddle%202) "1.000000,1.000000,1.000000")))
  (Actor|DestroyActor))

(event EventBeginPlay
  (bind _outactors (Actor|GetAllActorsOfClass "/Game/Blueprints/P1_Paddle.P1_Paddle_C"))
  (Variables|Default|SetPaddle%201 (Utilities|Array|Get(acopy) _outactors))
  (bind _outactors_2 (Actor|GetAllActorsOfClass "/Game/Blueprints/P2_Paddle.P2_Paddle_C"))
  (Variables|Default|SetPaddle%202 (Utilities|Array|Get(acopy) _outactors_2)))

(fn ConstructionScript)

(fn ChangeScale
  (params (Scale%20Value :type Vector))
  (Transformation|SetActorScale3D Scale%20Value))