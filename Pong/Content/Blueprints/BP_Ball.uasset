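; BP_Ball is the physics-driven ball for a two-player Pong-style game, launched along Y on BeginPlay.
; Overlaps pass through a chain of cast-based sub-graphs for each paddle, walls and each goal, falling through on failed casts.
; Paddle hits reset velocity using paddle X speed plus random spread and apply opposing forces, while walls invert X velocity.
; Goals recenter the ball and relaunch it along Y, without any scoring.
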(event EventBeginPlay
  (Physics|SetPhysicsLinearVelocity (Variables|Default|GetBall) "0,600.000000, 0" false "None"))

(event Collision|EventActorBeginOverlap
  (params (OtherActor :type Actor%20Object%20Reference))
  (|Paddle1 OtherActor
    (:CastFailed
      (|Paddle2 OtherActor
        (:CastFailed
          (|Walls OtherActor
            (:CastFailed
              (|Player1Goal OtherActor
                (:CastFailed
                  (|Player2Goal OtherActor))))))))))

(fn ConstructionScript)