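; Player 1's paddle actor, driven along the X axis by player input.
; Each tick it scales the Player1_MovingOnUp value and passes it to Move, which applies it as a physics force on the Paddle component.
; On reaching either hard-coded X limit, it is instead snapped just inside the boundary and receives no force that tick.
; A separate ChangeSCALE function sets the actor's scale.
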(event EventTick
  (params (DeltaSeconds :type Float%20%28single-precision%29))
  (bind _returnvalue (Transformation|GetActorLocation))
  (bind _returnvalue_2 (Transformation|GetActorLocation))
  (bind (_x _y _z) (Math|Vector|BreakVector _returnvalue))
  (bind (_x_2 _y_2 _z_2) (Math|Vector|BreakVector _returnvalue_2))
  ;[1 1 1] When Paddle Becomes More Than 399 Set's Actor Location To 398
  (if (>= (.X (Math|Vector|BreakVector (Transformation|GetActorLocation))) 399.0)
    (Transformation|SetActorLocation (Math|Vector|MakeVector 398.0 _y _z) false false)
    (elif (<= (.X (Math|Vector|BreakVector (Transformation|GetActorLocation))) -399.0)
      ;[1 1 1] Comment
      (Transformation|SetActorLocation (Math|Vector|MakeVector -398.0 _y_2 _z_2) false false)
      (else
        ;[1 1 1] Adds A Vector of 200000 To The Paddle To Make It Move
        (CallFunction|Move (* (Input|AxisValues|GetPlayer1_MovingOnUp) 8e+03))))))

(fn ConstructionScript)

(fn ChangeSCALE
  (params (Scale%20Value :type Vector))
  (Transformation|SetActorScale3D Scale%20Value))

(fn Move
  (params (Force :type Float%20%28single-precision%29))
  (Physics|AddForce (Variables|Default|GetPaddle) (Math|Vector|MakeVector Force 0.0 0.0) "None" false))