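; Pickup spawn area actor that scatters paddle, ball and third-person pickups inside a box volume.
; When IfVisible is set, the construction script calls one spawn function per pickup type: enlarge paddle, shrink paddle, shrink ball, third person and enlarge ball.
; Each function adds a child actor component at a random point within the PickUpArea box, so placement is rolled at construction rather than during play.
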(fn ConstructionScript
  (if (Variables|Default|GetIfVisible)
    (CallFunction|SpawnPickup-EnlargePaddle)
    (CallFunction|SpawnPickup-ShrinkPaddle)
    (CallFunction|SpawnPickup-ShrinkBall)
    (CallFunction|SpawnPickup-ThirdPerson)
    (CallFunction|SpawnPickup-EnlargeBall)))

(fn SpawnPickup-EnlargePaddle
  (bind _pickuparea (Variables|Default|GetPickUpArea))
  (AddComponent|AddChildActorComponent false (Math|Conversions|ToTransform(Vector) (Math|Random|RandomPointinBoundingBox (Variables|/Script/Engine.SceneComponent|GetRelativeLocation _pickuparea) (Variables|/Script/Engine.BoxComponent|GetBoxExtent _pickuparea)))))

(fn SpawnPickup-ShrinkPaddle
  (bind _pickuparea (Variables|Default|GetPickUpArea))
  (AddComponent|AddChildActorComponent false (Math|Conversions|ToTransform(Vector) (Math|Random|RandomPointinBoundingBox (Variables|/Script/Engine.SceneComponent|GetRelativeLocation _pickuparea) (Variables|/Script/Engine.BoxComponent|GetBoxExtent _pickuparea)))))

(fn SpawnPickup-ShrinkBall
  (bind _pickuparea (Variables|Default|GetPickUpArea))
  (AddComponent|AddChildActorComponent false (Math|Conversions|ToTransform(Vector) (Math|Random|RandomPointinBoundingBox (Variables|/Script/Engine.SceneComponent|GetRelativeLocation _pickuparea) (Variables|/Script/Engine.BoxComponent|GetBoxExtent _pickuparea)))))

(fn SpawnPickup-ThirdPerson
  (bind _pickuparea (Variables|Default|GetPickUpArea))
  (AddComponent|AddChildActorComponent false (Math|Conversions|ToTransform(Vector) (Math|Random|RandomPointinBoundingBox (Variables|/Script/Engine.SceneComponent|GetRelativeLocation _pickuparea) (Variables|/Script/Engine.BoxComponent|GetBoxExtent _pickuparea)))))

(fn SpawnPickup-EnlargeBall
  (bind _pickuparea (Variables|Default|GetPickUpArea))
  (AddComponent|AddChildActorComponent false (Math|Conversions|ToTransform(Vector) (Math|Random|RandomPointinBoundingBox (Variables|/Script/Engine.SceneComponent|GetRelativeLocation _pickuparea) (Variables|/Script/Engine.BoxComponent|GetBoxExtent _pickuparea)))))