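; ArduinoBlueprint turns slider input, apparently from an Arduino controller, into movement of the first P1_Paddle actor.
; Each Tick it maps the first ControllerValues entry from a 0–1023 range to -1..1, then refills that array by splitting Str on commas, so the slider uses the previously parsed data.
; It looks up the paddle every frame and calls Move with the scaled value; nothing here sets Str.
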(event EventBeginPlay)

(event Collision|EventActorBeginOverlap
  (params (OtherActor :type Actor%20Object%20Reference)))

(event EventTick
  (params (DeltaSeconds :type Float%20%28single-precision%29))
  (Variables|Default|SetSlider1Value (/ (- (Math|Conversions|ToFloat(Integer) (Utilities|Array|Get(acopy) (Variables|Default|GetController%20Values))) 511.5) 511.5))
  (Variables|Default|SetController%20Values (Utilities|String|ParseIntoArray (Variables|Default|Getstr) ","))
  (bind _outactors (Actor|GetAllActorsOfClass "/Game/Blueprints/P1_Paddle.P1_Paddle_C"))
  (Variables|Default|SetPaddle_1 (Utilities|Array|Get(acopy) _outactors))
  (Default|Move (Variables|Default|GetPaddle_1) (* (Variables|Default|GetSlider1Value) 8e+03)))

(fn ConstructionScript)